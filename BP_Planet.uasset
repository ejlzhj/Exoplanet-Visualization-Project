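; BP_Planet is a planet actor that takes its name, size and position from a data table.
; The construction script places and scales the Sphere from the current AngDist and PlanetScale values.
; BeginPlay loops every table row, overwriting those variables and adding a manually attached component per row at that distance and scale.
; Parent attachment, spring-arm distance and rotation rate logic exist but are unwired.
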(event EventBeginPlay
  (bind _table (Variables|Default|GetTable))
  (bind _outrownames (DataTable|GetDataTableRowNames _table))
  (for _array_element _outrownames
    (bind _returnvalue (Utilities|GetDataTableRow _table _array_element)
      (:then
        (Variables|Default|SetName (.name (Utilities|Struct|BreakTestData _returnvalue)))
        (bind _output_get (Variables|Default|SetPlanetScale (Math|Conversions|ToVector(Float) (.radius (Utilities|Struct|BreakTestData _returnvalue)))))
        (bind _output_get_2 (Variables|Default|SetAngDist (.angular_distance (Utilities|Struct|BreakTestData _returnvalue))))
        (AddComponent|AddSceneComponent true (Math|Transform|MakeTransform _output_get_2 "0, 0, 0" _output_get))))))

(event Collision|EventActorBeginOverlap
  (params (OtherActor :type Actor%20Object%20Reference)))

(event EventTick
  (params (DeltaSeconds :type Float%20%28single-precision%29)))

(fn ConstructionScript
  (Transformation|SetWorldLocation (Variables|Default|GetSphere) (Variables|Default|GetAngDist) false false)
  (Transformation|SetWorldScale3D (Variables|Default|GetSphere) (Variables|Default|GetPlanetScale))
  (Variables|Default|SetName (Variables|Default|GetName)))